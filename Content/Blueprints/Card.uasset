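; Card actor that shows a picture loaded from a JPG file on disk on its mesh.
; InitializeCard runs from both the construction script and BeginPlay, creating a dynamic material from Card_Mat_Parent on element 1 of CardMesh.
; LoadImage joins ImageDir to a hardcoded file name, prints the path, and loads it through the Victory plugin.
; The resulting texture feeds the material's TexturePicture parameter.
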(event EventBeginPlay
  (CallFunction|InitializeCard))

(event Collision|EventActorBeginOverlap
  (params (OtherActor :type Actor%20Object%20Reference)))

(event EventTick
  (params (DeltaSeconds :type Float%20%28single-precision%29)))

(fn ConstructionScript
  (CallFunction|InitializeCard))

(fn InitializeCard
  (bind _returnvalue (Rendering|Material|CreateDynamicMaterialInstance (Variables|Default|GetCardMesh) 1 "/Game/Materials/Card_Mat_Parent.Card_Mat_Parent" :!class /Script/Engine.PrimitiveComponent))
  (Variables|Default|SetDynamicPictureMaterial _returnvalue)
  (bind _imagetexture (CallFunction|LoadImage "\\image.jpg"))
  (Rendering|Material|SetTextureParameterValue (Variables|Default|GetDynamicPictureMaterial) "TexturePicture" _imagetexture))

(fn LoadImage
  (params (ImageName :type String))
  (bind _imagedir (Variables|Default|GetImageDir))
  (bind _returnvalue (Utilities|String|Append _imagedir ImageName))
  (Development|PrintString _returnvalue true true "(R=0.000000,G=0.660000,B=1.000000,A=1.000000)" 2e+01)
  (return (.ReturnValue (Class|VictoryBPFunctionLibrary|VictoryLoadTexture2DfromFile _returnvalue "JPG"))))